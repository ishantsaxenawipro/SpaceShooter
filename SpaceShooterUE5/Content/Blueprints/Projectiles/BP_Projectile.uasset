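; Projectile actor that damages what it hits, with a special path for flying pawns.
; On BeginPlay it adds AddedSpeed to the movement component's InitialSpeed, then destroys itself when its lifetime runs out.
; Hits on anything but its owner call TakeDamage on a BP_FlyingPawn or the generic ApplyDamage on other actors, then destroy the projectile.
; Debug strings print along the hit path.
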(event `self.ReceiveBeginPlay`
  (bind _projectilemovement (`self.ProjectileMovement`))
  (set `ProjectileMovementComponent.InitialSpeed` (+ (`self.AddedSpeed`) (`ProjectileMovementComponent.InitialSpeed` _projectilemovement)) _projectilemovement)
  (`KismetSystemLibrary.Delay` (`self.BulletLifetImeSeconds`))
  (`self.K2_DestroyActor`))

(event `self.ReceiveHit`
  (params (MyComp :type "PrimitiveComponent Object Reference") (Other :type "Actor Object Reference") (OtherComp :type "PrimitiveComponent Object Reference") (bSelfMoved :type Boolean) (HitLocation :type "Vector Structure") (HitNormal :type "Vector Structure") (NormalImpulse :type "Vector Structure") (Hit :type "HitResult Structure (by ref)"))
  (bind _damage (`self.Damage`))
  (`KismetSystemLibrary.PrintString` "Hit")
  (if (not (== Other (`self.GetOwner`)))
    (bind _asbp_flying_pawn (cast `/Game/Blueprints/BP_FlyingPawn` Other)
      (:`then`
        (`KismetSystemLibrary.PrintString` "Damaging Player")
        (`/Game/Blueprints/BP_FlyingPawn.Take Damage` _asbp_flying_pawn _damage))
      (:`CastFailed`
        (`KismetSystemLibrary.PrintString` "Damagin What So Ever!!")
        (`GameplayStatics.ApplyDamage` Other _damage null null "/Script/Engine.DamageType")))
    (`KismetSystemLibrary.PrintString` "Projectile Attacked")
    (`self.K2_DestroyActor`)))

(fn `UserConstructionScript`)