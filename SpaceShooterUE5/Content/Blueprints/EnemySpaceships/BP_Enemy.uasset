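; Enemy spaceship for the flying game mode that turns to face the player and fires at them when within shooting range.
; Tick updates yaw and clamped roll, then either spawns projectiles from the two gun sockets or runs down the fire-rate cooldown.
; Any damage removes a fixed amount of health, destroying the ship at zero.
; BeginPlay and death adjust the game mode's AliveEnemies count.
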(event `self.ReceiveBeginPlay`
  (set `self.PlayerPawn` (`GameplayStatics.GetPlayerPawn` 0))
  (set `self.CanShoot` true)
  (set `self.Count Down` (`self.FireRate`))
  (bind _asbp_flying_game_mode (cast `/Game/Blueprints/BP_FlyingGameMode` (`GameplayStatics.GetGameMode`)))
  (set `/Game/Blueprints/BP_FlyingGameMode.AliveEnemies` (+ (`/Game/Blueprints/BP_FlyingGameMode.AliveEnemies` _asbp_flying_game_mode) 1) _asbp_flying_game_mode))

(event `self.ReceiveTick`
  (params (DeltaSeconds :type "Float (single-precision)"))
  (bind _playerpawn (`self.PlayerPawn`))
  (bind _count_down (`self.Count Down`))
  (bind _returnvalue (`KismetStringLibrary.Conv_DoubleToString` (`self.Count Down`)))
  (`self.LookTowardPlayer` _playerpawn _playerpawn)
  (bind _inrange (`self.InRange` _playerpawn))
  (if (and (`self.CanShoot`) _inrange)
    (`self.Shoot`)
    (else
      (set `self.Count Down` (- _count_down DeltaSeconds))
      (if (<= _count_down 0.0)
        (set `self.CanShoot` true)
        (set `self.Count Down` (`self.FireRate`))
        (`KismetSystemLibrary.PrintString` "Can Shoot Now")
        (`KismetSystemLibrary.PrintString` _returnvalue)
        (else
          (`KismetSystemLibrary.PrintString` "Cant Shoot")
          (`KismetSystemLibrary.PrintString` "Count Down")
          (`KismetSystemLibrary.PrintString` _returnvalue))))))

(event `self.ReceiveAnyDamage`
  (params (Damage :type "Float (single-precision)") (DamageType :type "DamageType Object Reference") (InstigatedBy :type "Controller Object Reference") (DamageCauser :type "Actor Object Reference"))
  (bind _health (`self.Health`))
  (set `self.Health` (- _health 10.0))
  (if (<= _health 0.0)
    (`KismetSystemLibrary.PrintString` "EnemyHealth")
    (`KismetSystemLibrary.PrintString` (`KismetStringLibrary.Conv_DoubleToString` _health))
    (`GameplayStatics.PlaySound2D` "/Game/Audio/SpaceShipDestroyed.SpaceShipDestroyed" 1.0 1.0 0.0 null null)
    (bind _asbp_flying_game_mode (cast `/Game/Blueprints/BP_FlyingGameMode` (`GameplayStatics.GetGameMode`))
      (:`then`
        (set `/Game/Blueprints/BP_FlyingGameMode.AliveEnemies` (- (`/Game/Blueprints/BP_FlyingGameMode.AliveEnemies` _asbp_flying_game_mode) 1) _asbp_flying_game_mode))
      (:`CastFailed`
        _))
    (`self.K2_DestroyActor`)
    (else
      (`KismetSystemLibrary.PrintString` "EnemyHealth")
      (`KismetSystemLibrary.PrintString` (`KismetStringLibrary.Conv_DoubleToString` _health))
      (`GameplayStatics.PlaySound2D` "/Game/Audio/SpaceShip_Hit.SpaceShip_Hit" 1.0 1.0 0.0 null null))))

(fn `InRange`
  (params (Player :type "Pawn Object Reference"))
  (returns (inRange :type Boolean))
  (if (<= (`KismetMathLibrary.Vector_Distance` (`self.K2_GetActorLocation`) (`self.K2_GetActorLocation` Player)) (`self.ShootingRange`))
    (return true)
    (else
      (return false))))

(fn `LookTowardPlayer`
  (params (PlayerActor :type "Actor Object Reference") (Object :type "Object Object Reference"))
  (bind (_returnvalue_roll _returnvalue_pitch _returnvalue_yaw) (`KismetMathLibrary.BreakRotator` (`KismetMathLibrary.FindLookAtRotation` (`self.K2_GetActorLocation`) (`self.K2_GetActorLocation` PlayerActor))))
  (if (`KismetSystemLibrary.IsValid` Object)
    (`self.K2_SetActorRotation` (`KismetMathLibrary.MakeRotator` (`KismetMathLibrary.ClampAngle` _returnvalue_roll -80.0 80.0) 0.0 _returnvalue_yaw) true)))

(fn `Shoot`
  (bind _bulletscalefactor (`self.BulletScaleFactor`))
  (bind _projectilespeed (`self.ProjectileSpeed`))
  (bind (_returnvalue_location _returnvalue_rotation) (`KismetMathLibrary.BreakTransform` (`SceneComponent.GetSocketTransform` (`self.StaticMesh`) "GunR" "RTS_World")))
  (bind (_returnvalue_location_2 _returnvalue_rotation_2) (`KismetMathLibrary.BreakTransform` (`SceneComponent.GetSocketTransform` (`self.StaticMesh`) "GunL" "RTS_World")))
  (`|SpawnActorFromClass` "/Game/Blueprints/Projectiles/BP_Child_EnemyProjectile.BP_Child_EnemyProjectile_C" (`KismetMathLibrary.MakeTransform` _returnvalue_location_2 _returnvalue_rotation_2 (`KismetMathLibrary.Conv_DoubleToVector` _bulletscalefactor)) "Undefined" "OverrideRootScale" null _projectilespeed null)
  (`|SpawnActorFromClass` "/Game/Blueprints/Projectiles/BP_Child_EnemyProjectile.BP_Child_EnemyProjectile_C" (`KismetMathLibrary.MakeTransform` _returnvalue_location _returnvalue_rotation (`KismetMathLibrary.Conv_DoubleToVector` _bulletscalefactor)) "Undefined" "OverrideRootScale" null _projectilespeed null)
  (set `self.CanShoot` false)
  (`GameplayStatics.PlaySound2D` "/Game/Audio/heat-vision.heat-vision" 1.0 1.0 0.0 null null))

(fn `UserConstructionScript`)