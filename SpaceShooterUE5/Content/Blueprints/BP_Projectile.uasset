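; Projectile actor that deals damage to whatever it hits, other than its owner, then destroys itself.
; On BeginPlay it adds AddedSpeed to the ProjectileMovement component's InitialSpeed and destroys itself after a fixed delay if still alive.
; Its Hit event applies the configured Damage and DamageType to the other actor, ignoring hits on the owner.
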(event `self.ReceiveBeginPlay`
  (bind _projectilemovement (`self.ProjectileMovement`))
  (set `ProjectileMovementComponent.InitialSpeed` (+ (`self.AddedSpeed`) (`ProjectileMovementComponent.InitialSpeed` _projectilemovement)) _projectilemovement)
  (`KismetSystemLibrary.Delay` 20.0)
  (`self.K2_DestroyActor`))

(event `self.ReceiveHit`
  (params (MyComp :type "PrimitiveComponent Object Reference") (Other :type "Actor Object Reference") (OtherComp :type "PrimitiveComponent Object Reference") (bSelfMoved :type Boolean) (HitLocation :type "Vector Structure") (HitNormal :type "Vector Structure") (NormalImpulse :type "Vector Structure") (Hit :type "HitResult Structure (by ref)"))
  (if (not (== Other (`self.GetOwner`)))
    (`GameplayStatics.ApplyDamage` Other (`self.Damage`) null null "/Script/Engine.DamageType")
    (`self.K2_DestroyActor`)))

(fn `UserConstructionScript`)