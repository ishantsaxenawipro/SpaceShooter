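; Actor that builds a ring of instanced asteroids and slowly spins it around its local Z axis at RotationSpeed.
; The construction script loops over length and width counts, adding instances to a hierarchical instanced static mesh with cull distances.
; AsteroidTransformation spreads instances around the ring radius and width, using a seeded stream to jitter position and blend rotation toward random.
; Instance scale grows with width index rather than being random.
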(event `self.ReceiveTick`
  (params (DeltaSeconds :type "Float (single-precision)"))
  (`self.K2_AddActorLocalRotation` (`KismetMathLibrary.RotatorFromAxisAndAngle` (0.0 0.0 1.0) (* DeltaSeconds (`self.RotationSpeed`)))))

(fn `AsteroidTransformation`
  (params (IndexFromWidthLoop :type Integer) (NumberOfInstancesByWidth :type Integer) (IndexFromLengthLoop :type Integer) (NumberOfInstancesByLength :type Integer))
  (returns (OutLocation :type "Vector Structure") (OutRotation :type "Rotator Structure"))
  (bind _returnvalue (`KismetMathLibrary.MakeVector` 0.0 0.0 1.0))
  (bind _transformrandom (`self.TransformRandom`))
  (bind _returnvalue_2 (`KismetMathLibrary.RotateAngleAxis` (+ (+ (* (- (`KismetMathLibrary.RandomFloatFromStream` _transformrandom) 0.5) (`self.RandomizeZAxisPosition`) (`self.RingWidth`)) (* (`KismetMathLibrary.RandomUnitVectorFromStream` _transformrandom) (`self.RandomizePosition`))) (`KismetMathLibrary.MakeVector` 0.0 (+ (`self.RingRadius`) (* (- (/ (`KismetMathLibrary.Conv_IntToDouble` IndexFromWidthLoop) (`KismetMathLibrary.Conv_IntToDouble` NumberOfInstancesByWidth)) 0.5) (`self.RingWidth`))))) (* (/ (`KismetMathLibrary.Conv_IntToDouble` IndexFromLengthLoop) (`KismetMathLibrary.Conv_IntToDouble` NumberOfInstancesByLength)) 360.0) _returnvalue))
  (return _returnvalue_2 (`KismetMathLibrary.RLerp` (`KismetMathLibrary.MakeRotFromYZ` (`KismetMathLibrary.Cross_VectorVector` _returnvalue _returnvalue_2) _returnvalue) (`KismetMathLibrary.RandomRotatorFromStream` true (`self.TransformRandom`)) (`self.RandomizeRotation`) true)))

(fn `UserConstructionScript`
  (bind _hierarchicalinstancedstaticspawn (`self.HierarchicalInstancedStaticSpawn`))
  (bind _instancecountbylength (`self.InstanceCountByLength`))
  (bind _instancecountbywidth (`self.InstanceCountByWidth`))
  (`|ExecutionSequence`
    (:`then_0`
      (`StaticMeshComponent.SetStaticMesh` _hierarchicalinstancedstaticspawn (`self.InstanceMesh`)))
    (:`then_1`
      (`InstancedStaticMeshComponent.SetCullDistances` _hierarchicalinstancedstaticspawn (`self.CulligNear`) (`self.CulligFar`)))
    (:`then_2`
      (for _index (range _instancecountbylength)
        (for _index_2 (range _instancecountbywidth)
          (bind (_outlocation _outrotation) (`self.AsteroidTransformation` _index_2 _instancecountbywidth _index _instancecountbylength))
          (`InstancedStaticMeshComponent.AddInstance` (`self.HierarchicalInstancedStaticSpawn`) (`KismetMathLibrary.MakeTransform` _outlocation _outrotation (`KismetMathLibrary.Conv_DoubleToVector` (* (`self.RandomizeSacleMin`) _index_2))) false))))))