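; Enemy projectile Blueprint that damages the player's flying pawn on impact.
; On Hit it ignores its owner, casts the other actor to BP_FlyingPawn, calls that pawn's TakeDamage with its Damage value, then destroys itself.
; Hits on any other actor leave the projectile alive.
; Debug prints mark hits, and an unconnected ApplyDamage node is left unused.
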(event `self.ReceiveBeginPlay`
  (`parent.ReceiveBeginPlay`))

(event `self.ReceiveHit`
  (params (MyComp :type "PrimitiveComponent Object Reference") (Other :type "Actor Object Reference") (OtherComp :type "PrimitiveComponent Object Reference") (bSelfMoved :type Boolean) (HitLocation :type "Vector Structure") (HitNormal :type "Vector Structure") (NormalImpulse :type "Vector Structure") (Hit :type "HitResult Structure (by ref)"))
  (`KismetSystemLibrary.PrintString` "Enemy P Hit")
  (if (not (== Other (`self.GetOwner`)))
    (bind _asbp_flying_pawn (cast `/Game/Blueprints/BP_FlyingPawn` Other))
    (`/Game/Blueprints/BP_FlyingPawn.Take Damage` _asbp_flying_pawn (`self.Damage`))
    (`KismetSystemLibrary.PrintString` "Enemy Projectile Attaked")
    (`self.K2_DestroyActor`)))

(fn `UserConstructionScript`
  (`parent.UserConstructionScript`))